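; BP_EnemyAI is an overworld enemy that chases the player and switches the game to a battle scene on contact.
; PawnSensing sets a sight flag, never cleared here, and triggers an AI MoveTo toward the first player character.
; A capsule hit against bp_papercharacter opens the referenced level, passing DestinationTag as the options string.
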(event `self.PawnSensing.OnSeePawn`
  (params (Pawn :type "Pawn Object Reference"))
  ;[1 1 1] Chase Player
  (set `self.CanSeePlayer` true)
  (`self.FollowPlayer`))

(event `FollowPlayer`
  ;[1 1 1] Chase Player
  (if (`self.CanSeePlayer`)
    (`|AIMoveTo` self (0.0 0.0 0.0) (`GameplayStatics.GetPlayerCharacter` 0))))

(event `self.CapsuleComponent.OnComponentHit`
  (params (HitComponent :type "PrimitiveComponent Object Reference") (OtherActor :type "Actor Object Reference") (OtherComp :type "PrimitiveComponent Object Reference") (NormalImpulse :type "Vector Structure") (Hit :type "HitResult Structure (by ref)"))
  ;[1 1 1] switch to battle scene
  (cast `/Game/PlayerCharacter/Blueprints/bp_papercharacter` OtherActor)
  (`GameplayStatics.OpenLevelBySoftObjectPtr` (`self.Level`) true (`self.DestinationTag`)))

(fn `UserConstructionScript`)